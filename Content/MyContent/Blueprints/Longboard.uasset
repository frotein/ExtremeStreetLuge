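; Longboard actor with a board model and a RotationPoint pivot that rolls at a constant, delta-time-scaled rate on Tick.
; GetPosition and GetRotation expose the pivot's world transform.
; RotateBoard adds a rotation to BoardModel and uses RotateAround to place it along the new up vector from the pivot, offset by the pivot's relative-location length.
; RotateBoard also prints the pivot location and is not called within this Blueprint.
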(event EventBeginPlay)

(event EventActorBeginOverlap
  (params (OtherActor :type Actor%20Object%20Reference)))

(event EventTick
  (params (DeltaSeconds :type Float%20%28single-precision%29))
  (Transformation|AddRelativeRotation (Variables|Default|GetrotationPoint) (Math|Rotator|MakeRotator (* 20 DeltaSeconds) 0.0 0.0) false false))

(fn ConstructionScript)

(fn GetPosition
  (return (Transformation|GetWorldLocation (Variables|Default|GetrotationPoint))))

(fn GetRotation
  (return (Transformation|GetWorldRotation (Variables|Default|GetrotationPoint))))

(fn RotateAround
  (params (rotation :type Rotator) (distance :type Float%20%28single-precision%29) (center :type Vector))
  (return (+ center (* (Math|Vector|GetUpVector rotation) distance))))

(fn RotateBoard
  (params (additionalRotation :type Rotator))
  (bind _board_model (Variables|Default|GetBoard%20Model))
  (bind _rotationpoint (Variables|Default|GetrotationPoint))
  (bind _returnvalue (Transformation|GetWorldRotation _board_model))
  (bind _returnvalue_2 (Transformation|GetWorldLocation _rotationpoint))
  (bind _returnvalue_3 (Math|Rotator|CombineRotators _returnvalue additionalRotation))
  (Development|PrintString (Utilities|String|ToString(Vector) _returnvalue_2))
  (Transformation|SetWorldLocationAndRotation _board_model (CallFunction|RotateAround _returnvalue_3 (Math|Vector|VectorLength (Variables|/Script/Engine.SceneComponent|GetRelativeLocation _rotationpoint)) _returnvalue_2) _returnvalue_3 false false))